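; Shooting range minigame that starts when a non-bot pawn enters its box and stops, resetting targets, when that pawn leaves.
; A looping timer randomly activates one or two timed targets until the session total is reached, with hits scoring by time left.
; Accuracy from hits versus PlayerState bullets fired adds a score bonus, and records persist in a BP_Trial_ScoreSave slot.
; A session widget shows live counters and final results.
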(event OnComponentBeginOverlap(Box)
  (params (OverlappedComponent :type Primitive%20Component%20Object%20Reference) (OtherActor :type Actor%20Object%20Reference) (OtherComp :type Primitive%20Component%20Object%20Reference) (OtherBodyIndex :type Integer) (bFromSweep :type Boolean) (SweepResult :type Hit%20Result%20Structure%20%28by%20ref%29))
  ;[0 0 0] Start Minigame on Overlap
  (bind _aspawn (Utilities|Casting|CastToPawn OtherActor))
  (if (not (Variables|/Script/Engine.PlayerState|GetbIsABot (Variables|/Script/Engine.Pawn|GetPlayerState _aspawn)))
    (Variables|Default|SetAs%20Pawn _aspawn)
    (CallFunction|StartMinigame)
    (Utilities|IsValid (Variables|Default|GetWB_ShootingRange)
      (:Is%20Valid
        (Widget|RemovefromParent (Variables|Default|GetWB_ShootingRange)))
      (:Is%20Not%20Valid
        _))
    (bind _returnvalue (UserInterface|CreateWidget "/Game/FPS_Controller/UI/Trial/WB_ShootingRangeSession.WB_ShootingRangeSession_C" (Game|GetPlayerController 0)))
    (bind _output_get (Variables|Default|SetWB_ShootingRange _returnvalue))
    (UserInterface|Viewport|AddtoViewport _output_get 0)))

(event OnComponentEndOverlap(Box)
  (params (OverlappedComponent :type Primitive%20Component%20Object%20Reference) (OtherActor :type Actor%20Object%20Reference) (OtherComp :type Primitive%20Component%20Object%20Reference) (OtherBodyIndex :type Integer))
  ;[0 0 0] Exit minigame
  (if (== OtherActor (Variables|Default|GetAs%20Pawn))
    (for _array_element (Variables|Default|GetShootingRangeTargets)
      (Utilities|IsValid _array_element
        (:Is%20Valid
          (Default|ResetDummyPosition _array_element))))
    (Utilities|Time|ClearandInvalidateTimerbyHandle (Variables|Default|GetShhotingRangeTimerHandle))
    (Widget|RemovefromParent (Variables|Default|GetWB_ShootingRange))))

(event Custom|StartMinigame
  ;[0 0 0] Start Minigame
  (CallFunction|LoadPreviousRecords)
  (CallFunction|InitMinigame)
  (Audio|PlaySound2D "/Engine/VREditor/Sounds/VR_negative_Cue.VR_negative_Cue" 1.0 1.0 0.0 0 0)
  (bind _returnvalue (Utilities|Time|SetTimerbyEvent (delegate Custom|ActivateTarget) 1.7 true))
  (Variables|Default|SetShhotingRangeTimerHandle _returnvalue))

(event Custom|EndShootingRangeSession
  ;[0 0 0] End Shooting range session
  (CallFunction|CalculateAccuracy)
  (CallFunction|CalculateFinalScore)
  (Default|ShowResults (Variables|Default|GetWB_ShootingRange) (Variables|Default|GetBonusScore) (Variables|Default|GetFinalScore) (Variables|Default|GetAccuracy) (Variables|Default|GetRecordScore)))

(event Custom|Calculate%20Accuracy
  ;[0 0 0] Calculate Accuracy
  (bind _bulletsfired (Class|BIPlayerState|GetBulletsFired(Message) (Variables|/Script/Engine.Controller|GetPlayerState (Game|GetPlayerController 0))))
  (Variables|Default|SetAccuracy (* (/ (Math|Conversions|ToFloat(Integer) (Variables|Default|GetTargetsHit)) (Math|Conversions|ToFloat(Integer) (- _bulletsfired (Variables|Default|GetBulletsFiredStart)))) 1e+02)))

(event Custom|SetShootingRangeRecord
  (params (New%20Score :type Integer))
  ;[0 0 0] Set new record
  (bind _returnvalue (SaveGame|CreateSaveGameObject "/Game/FPS_Controller/Blueprints/SaveGame/BP_Trial_ScoreSave.BP_Trial_ScoreSave_C"))
  (bind _output_get (Variables|/Game/FPS_Controller/Blueprints/SaveGame/BP_Trial_ScoreSave.BP_Trial_ScoreSave_C|SetRecordScore _returnvalue New%20Score))
  (Variables|Default|SetRecordScore _output_get)
  (SaveGame|SaveGametoSlot _returnvalue "Save"))

(event Custom|InitMinigame
  ;[0 0 0] Init Minigame
  (bind _bulletsfired (Class|BIPlayerState|GetBulletsFired(Message) (Variables|/Script/Engine.Controller|GetPlayerState (Game|GetPlayerController 0))))
  (Variables|Default|SetBulletsFiredStart _bulletsfired)
  (Variables|Default|SetScore 0)
  (Variables|Default|SetTargetsUsed 0)
  (Variables|Default|SetTargetsHit 0))

(event Custom|Calculate%20Final%20Score
  (bind _score (Variables|Default|GetScore))
  (bind _accuracy (Variables|Default|GetAccuracy))
  (bind _returnvalue (/ _accuracy 1e+02))
  (bind _returnvalue_2 (* _score _returnvalue))
  (bind _returnvalue_3 (Math|Float|Truncate _returnvalue_2))
  ;[0 0 0] Calculate Final Score
  (Variables|Default|SetBonusScore _returnvalue_3)
  (bind _output_get (Variables|Default|SetFinalScore (+ _score _returnvalue_3)))
  (if (< (Variables|Default|GetRecordScore) _output_get)
    (CallFunction|SetShootingRangeRecord _output_get)))

(event Custom|ActivateTarget
  (bind _shootingrangetargets (Variables|Default|GetShootingRangeTargets))
  (if (< (Variables|Default|GetTargetsUsed) (Variables|Default|GetSessionTotalTargets))
    (if (Math|Random|RandomBool)
      ;[0 0 0] Activate target
      (CallFunction|Activate (Utilities|Array|Get(acopy) _shootingrangetargets (Math|Random|RandomIntegerinRange 0 (Utilities|Array|LastIndex _shootingrangetargets))) (Variables|Default|GetTargetActiveTime))
      (else
        ;[0 0 0] Ativate 2 targets
        (Variables|Default|SetPossibleTargets (Variables|Default|GetShootingRangeTargets))
        (for _index (range 0 1)
          (if (< (Variables|Default|GetTargetsUsed) (Variables|Default|GetSessionTotalTargets))
            (bind _output_get (Variables|Default|SetSelectedTarget (Utilities|Array|Get(acopy) (Variables|Default|GetPossibleTargets) (Math|Random|RandomIntegerinRange 0 (Utilities|Array|LastIndex (Variables|Default|GetPossibleTargets))))))
            (CallFunction|Activate _output_get (Variables|Default|GetTargetActiveTime))
            (Utilities|Array|RemoveItem (Variables|Default|GetPossibleTargets) _output_get)))))
    (else
      ;[0 0 0] End Shooting range session
      (Utilities|Time|ClearandInvalidateTimerbyHandle (Variables|Default|GetShhotingRangeTimerHandle))
      (Utilities|FlowControl|Delay 2.0)
      (CallFunction|EndShootingRangeSession)
      (Audio|PlaySound2D "/Engine/VREditor/Sounds/VR_grab_Cue.VR_grab_Cue" 1.0 1.0 0.0 0 0))))

(event Custom|AddScore
  (params (TimeLeft :type Float%20%28double-precision%29))
  ;[0 0 0] Add Score
  (bind _output_get (Variables|Default|SetScore (+ (Variables|Default|GetScore) (Math|Float|Truncate (* TimeLeft 1e+03)))))
  (Default|UpdateTargetsCounter (Variables|Default|GetWB_ShootingRange) (Variables|Default|GetTargetsHit) (Variables|Default|GetTargetsUsed) _output_get))

(event Custom|LoadPreviousRecords
  ;[0 0 0] Load Record
  (bind _returnvalue (SaveGame|LoadGamefromSlot "Save"))
  (bind _asbp_trial_score_save (Utilities|Casting|CastToBP_Trial_ScoreSave _returnvalue)
    (:then
      (Variables|Default|SetRecordScore (Variables|/Game/FPS_Controller/Blueprints/SaveGame/BP_Trial_ScoreSave.BP_Trial_ScoreSave_C|GetRecordScore _asbp_trial_score_save)))
    (:CastFailed
      (SaveGame|CreateSaveGameObject "/Game/FPS_Controller/Blueprints/SaveGame/BP_Trial_ScoreSave.BP_Trial_ScoreSave_C")
      (Variables|Default|SetRecordScore 0))))

(event Custom|Activate
  (params (Target :type BP%20Base%20Target%20Object%20Reference) (Time :type Float%20%28double-precision%29))
  ;[0 0 0] Activate
  (EventDispatchers|AssignOnHit Target (delegate Custom|OnHit_Event))
  (Default|InitTarget Target)
  (Default|DelayDeactivate Target Time)
  (Variables|Default|SetTargetsUsed (+ (Variables|Default|GetTargetsUsed) 1))
  (Default|UpdateTargetsCounter (Variables|Default|GetWB_ShootingRange) (Variables|Default|GetTargetsHit) (Variables|Default|GetTargetsUsed) (Variables|Default|GetScore)))

(event Custom|OnHit_Event
  (params (TimeLeft :type Float%20%28double-precision%29))
  ;[0 0 0] Activate
  (CallFunction|AddScore TimeLeft)
  (Variables|Default|SetTargetsHit (+ (Variables|Default|GetTargetsHit) 1))
  (Default|UpdateTargetsCounter (Variables|Default|GetWB_ShootingRange) (Variables|Default|GetTargetsHit) (Variables|Default|GetTargetsUsed) (Variables|Default|GetScore)))

(fn ConstructionScript
  (Components|Box|SetBoxExtent (Variables|Default|GetBox) (Variables|Default|GetIn%20Box%20Extent) true))