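; BP_PreviewLethal is a preview actor that displays the lethal equipment mesh from the player's preview loadout.
; On BeginPlay it retries until the player controller is valid, then binds to AC_Loadout's preview-loadout-changed event.
; Each change re-reads the loadout and async loads the lethal's static mesh onto LethalMesh.
; It also carries attachment spawn and load helpers, which the event graph does not call.
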(event Custom|SetNewPreviewLoadout
  ;[0 0 0] Update Attachments
  (Variables|Default|SetPreview%20Loadout (Default|GetPreviewLoadout (Variables|Default|GetLoadoutComponent)))
  (CallFunction|UpdateWeapon))

(event Custom|UpdateWeapon
  (bind _preview_loadout (Variables|Default|GetPreview%20Loadout))
  (bind _lethalequipmentmesh (Variables|/Game/FPS_Controller/Blueprints/DataAssets/LethalEquippmentData/PDA_LethalEquippmentInfo.PDA_LethalEquippmentInfo_C|GetLethalEquipmentMesh (.lethalequipment _preview_loadout)))
  ;[0 0 0] Update Weapon
  (Utilities|AsyncLoadAsset _lethalequipmentmesh
    (:Completed
      (Components|StaticMesh|SetStaticMesh (Variables|Default|GetLethalMesh) (Utilities|ResolveSoftReference _lethalequipmentmesh)))))

(event Custom|PreviewLoadoutChanged_Event
  ;[0 0 0] Begin play
  (CallFunction|SetNewPreviewLoadout))

(event EventBeginPlay
  (bind _returnvalue (Game|GetPlayerController 0))
  ;[0 0 0] Begin play
  (Utilities|IsValid _returnvalue :!label _label ; ensure that the controller is valid
    (:Is%20Valid
      (bind _output_get (Variables|Default|SetController _returnvalue))
      (Variables|Default|SetLoadoutComponent (Actor|GetComponentbyClass _output_get "/Game/FPS_Controller/Blueprints/Components/AC_Loadout.AC_Loadout_C"))
      (EventDispatchers|AssignPreviewLoadoutChanged (Actor|GetComponentbyClass _output_get "/Game/FPS_Controller/Blueprints/Components/AC_Loadout.AC_Loadout_C") (delegate Custom|PreviewLoadoutChanged_Event)))
    (:Is%20Not%20Valid
      (Utilities|FlowControl|Delay 0.1)
      (goto _label))))

(fn ConstructionScript)

(fn Equipattachment
  (params (Default%20Attachment :type BP%20Base%20Attachment%20Class%20Reference) (Attachment :type BP%20Base%20Attachment%20Class%20Reference))
  (bind _returnvalue (Utilities|IsValidClass Attachment))
  (bind _returnvalue_2 (select _returnvalue Attachment Default%20Attachment))
  (if (Utilities|IsValidClass _returnvalue_2)
    (bind _returnvalue_3 (Game|SpawnActorfromClass _returnvalue_2 (Math|Transform|MakeTransform "0, 0, 0" "0, 0, 0" "1.000000,1.000000,1.000000") "AlwaysSpawn" "SelectDefaultAtRuntime" self 0))
    (LocalVariables|SetAttachmentRef _returnvalue_3)
    (Transformation|AttachComponentToComponent (Default|GetTPPMesh (LocalVariables|GetAttachmentRef)) 0 (Variables|/Game/FPS_Controller/Blueprints/Attachments/BP_Base_Attachment.BP_Base_Attachment_C|GetSocket (LocalVariables|GetAttachmentRef)) "SnapToTarget" "SnapToTarget" "SnapToTarget" true)
    (return (LocalVariables|GetAttachmentRef))))