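; BP_ExplosiveBarrel is a replicated explosive prop that takes damage through ACHealth, shows the instigator a hit marker, and explodes when dead.
; On death it wakes net dormancy and sets a RepNotify Destroyed flag, which hides the mesh, disables collision and removes the health component.
; The explosion waits one tick, applies radial damage credited to the instigator, multicasts effects, sound, camera shake and radial impulse, then sets a lifespan.
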(event Custom|Explode
  (params (Instigator :type Controller%20Object%20Reference))
  (bind _returnvalue (Transformation|GetActorLocation))
  (bind _self self)
  ;[0 0 0] Explode
  (Utilities|FlowControl|DelayUntilNextTick)
  (Game|Damage|ApplyRadialDamage 5e+02 (Math|Vector|MakeVector (.x _returnvalue) (.y _returnvalue) (+ (.z _returnvalue) 8e+01)) (Variables|Default|GetExplosionRadius) 0 (Utilities|Array|MakeArray _self) _self Instigator false "ECC_WorldDynamic")
  (CallFunction|MulticastPlayCosmeticEffects)
  (Actor|SetLifeSpan 25.0))

(event Custom|Multicast_PlayCosmeticEffects
  (bind _self self)
  (bind _explosionradius (Variables|Default|GetExplosionRadius))
  (bind _returnvalue (Transformation|GetActorLocation _self))
  (bind (_x _y _z) (Math|Vector|BreakVector _returnvalue))
  (bind _returnvalue_2 (+ _z 8e+01))
  (bind _returnvalue_3 (Math|Vector|MakeVector _x _y _returnvalue_2))
  ;[0 0 0] Play Cosmetic effects
  (Networking|CanExecuteCosmeticEvents
    (:True
      (Niagara|SpawnSystematLocation "/Game/FPS_Controller/Effects/Particles/NS_Grenade_Explosion.NS_Grenade_Explosion" _returnvalue_3)
      (Audio|PlaySoundatLocation "/Game/FPS_Controller/Audio/Explosions/SC_Explosions_Grenade_Noise-Interior-Distant_01_Cue.SC_Explosions_Grenade_Noise-Interior-Distant_01_Cue" _returnvalue_3 "0, 0, 0" 1.0 1.0 0.0 0 0 0 0)
      (Camera|PlayWorldCameraShake "/Game/FPS_Controller/Blueprints/CameraShakes/CS_Explosion.CS_Explosion_C" _returnvalue_3 (* _explosionradius 2.0) (* _explosionradius 3.0))
      (Class|RadialForceComponent|FireImpulse (Variables|Default|GetRadialForce)))))

(event Custom|Destroyed
  (bind _ac_health (Variables|Default|GetAC_Health))
  (bind _explosiveporpmesh (Variables|Default|GetExplosivePorpMesh))
  ;[0 0 0] Destroyed
  (Rendering|SetVisibility _explosiveporpmesh false false)
  (Collision|SetCollisionEnabled _explosiveporpmesh "NoCollision")
  (Utilities|IsValid _ac_health
    (:Is%20Valid
      (Components|DestroyComponent _ac_health))))

(event Game|Damage|EventAnyDamage
  (params (Damage :type Float%20%28single-precision%29) (DamageType :type Damage%20Type%20Object%20Reference) (InstigatedBy :type Controller%20Object%20Reference) (DamageCauser :type Actor%20Object%20Reference))
  (bind _ac_health (Variables|Default|GetAC_Health))
  ;[0 0 0] Any Damage
  (if (not (Variables|Default|GetbDestroyed))
    (Class|BIPawnActions|ShowHitMarker(Message) (Pawn|GetControlledPawn InstigatedBy) true)
    (Default|HandleDamage _ac_health Damage)
    (if (Default|IsDead _ac_health)
      (Networking|SetNetDormancy "DORM_Awake")
      (Variables|Default|SetbDestroyed true)
      (Networking|ForceNetUpdate)
      (CallFunction|Explode InstigatedBy))))

(fn ConstructionScript)

(fn OnRepBDestroyed
  (CallFunction|Destroyed))