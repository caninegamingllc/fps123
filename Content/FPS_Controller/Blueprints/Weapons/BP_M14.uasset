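; M14 weapon Blueprint that adds a Picatinny rail support mesh when certain attachments are fitted.
; Its construction script runs the parent's, then leaves the first- and third-person rail components empty.
; The attachment component's OnRepAttachment event assigns the support mesh to both for two attachment types.
; GetExtraMesh exposes the third-person rail's current mesh.
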(event OnRepAttachment(AC_WeaponAttachments)
  (params (Attachment :type BP%20Base%20Attachment%20Object%20Reference))
  (bind _type (Variables|/Game/FPS_Controller/Blueprints/Attachments/BP_Base_Attachment.BP_Base_Attachment_C|GetType Attachment))
  (Utilities|IsValid Attachment
    (:Is%20Valid
      (if (or (Utilities|Enum|Equal(Enum) _type "NewEnumerator1") (Utilities|Enum|Equal(Enum) _type "NewEnumerator6"))
        (Components|SkeletalMesh|SetSkeletalMeshAsset (Variables|Default|GetPicatinyFPP) (Variables|Default|GetPicatinySupportMesh))))))

(fn ConstructionScript
  (|CallParentFunction)
  (Components|SkeletalMesh|SetSkeletalMeshAsset (Variables|Default|GetPicatinyFPP) 0))

(fn GetExtraMesh
  (return (Variables|/Script/Engine.SkeletalMeshComponent|GetSkeletalMeshAsset (Variables|Default|GetPicatinyTPP))))