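; Base shooting-range dummy target that can be activated, hit once for scoring, or deactivated by a timer.
; Init_Target plays the activate animation and enables collision, while DelayDeactivate starts a timer that resets the target.
; Damage while active deactivates it, fires OnHit with the timer's remaining time for scoring, and notifies the shooter pawn's AC_PawnInfo.
; SetState keeps the Active flag and actor collision in sync.
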(event Custom|Init_Target
  ;[0 0 0] Ini Target
  (Components|Animation|PlayAnimation (Variables|Default|GetSkeletalMesh) (Variables|Default|GetActivate_Anim) false)
  (CallFunction|SetState true))

(event Custom|DelayDeactivate
  (params (Time :type Float%20%28double-precision%29))
  ;[0 0 0] On Target Activation we set a timer to deactivate it
  (bind _returnvalue (Utilities|Time|SetTimerbyEvent (delegate Custom|Reset%20Dummy%20Position) Time))
  (Variables|Default|SetTimeLeftHandle _returnvalue))

(event Custom|Reset%20Dummy%20Position
  ;[0 0 0] On Target Activation we set a timer to deactivate it
  (if (Variables|Default|GetbActive)
    (Components|Animation|PlayAnimation (Variables|Default|GetSkeletalMesh) (Variables|Default|GetOnHit_Anim) false))
  (CallFunction|SetState false))

(event Game|Damage|EventAnyDamage
  (params (Damage :type Float%20%28single-precision%29) (DamageType :type Damage%20Type%20Object%20Reference) (InstigatedBy :type Controller%20Object%20Reference) (DamageCauser :type Actor%20Object%20Reference))
  (bind _returnvalue (Pawn|GetControlledPawn InstigatedBy))
  (bind _timelefthandle (Variables|Default|GetTimeLeftHandle))
  (bind _returnvalue_2 (Actor|GetComponentbyClass _returnvalue "/Game/FPS_Controller/Blueprints/Components/AC_PawnInfo.AC_PawnInfo_C"))
  ;[0 0 0] On damage taken
  (if (Variables|Default|GetbActive)
    (Components|Animation|PlayAnimation (Variables|Default|GetSkeletalMesh) (Variables|Default|GetOnHit_Anim) false)
    (CallFunction|SetState false)
    (Utilities|FlowControl|Sequence
      (:then_0
        ;;[0.0625 0.0625 0.0625] Add Score
        (if (Utilities|Time|IsValidTimerHandle _timelefthandle)
          (Default|CallOnHit (Utilities|Time|GetTimerRemainingTimebyHandle _timelefthandle))
          (else
            (Default|CallOnHit 0.0))))
      (:then_1
        (Utilities|IsValid _returnvalue_2
          (:Is%20Valid
            (Default|CallOnDamageDone _returnvalue_2 true)))))))

(event EventBeginPlay
  ;[0 0 0] Begin Play
  (Components|Animation|PlayAnimation (Variables|Default|GetSkeletalMesh) (Variables|Default|GetDeactivated_Anim) false)
  (CallFunction|SetState false))

(fn ConstructionScript)

(fn SetState
  (params (bActive :type Boolean))
  (bind _output_get (Variables|Default|SetbActive bActive))
  (Collision|SetActorEnableCollision _output_get))