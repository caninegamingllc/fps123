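; Battle royale game mode that assigns joining players to squads and drives match phases through the game state.
; PostLogin fills squads and, at the minimum player count, starts a delayed countdown into the match.
; Elimination flags the player state and refreshes the alive count from total player count; match end records the winning squad and opens MainMenu, with no win check here.
; Spectating, knife equip and loot/zone spawning are print-only stubs.
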(event Custom|AssignSquadToController
  (params (NewPlayer :type Player%20Controller%20Object%20Reference))
  (bind _asbp_br_player_state (Utilities|Casting|CastToBP_BR_PlayerState (Variables|/Script/Engine.Controller|GetPlayerState NewPlayer)))
  (Variables|/Game/FPS_Controller/Blueprints/Game/BattleRoyale/BP_BR_PlayerState.BP_BR_PlayerState_C|SetSquadId _asbp_br_player_state (Variables|BattleRoyale|GetNextSquadId))
  (Development|PrintString "BR Squad Assigned")
  (Variables|BattleRoyale|SetCurrentSquadFill (+ (Variables|BattleRoyale|GetCurrentSquadFill) 1))
  (if (>= (+ (Variables|BattleRoyale|GetCurrentSquadFill) 1) (Variables|BattleRoyale|GetSquadSize))
    (Variables|BattleRoyale|SetNextSquadId (+ (Variables|BattleRoyale|GetNextSquadId) 1))
    (Variables|BattleRoyale|SetCurrentSquadFill 0))
  (CallFunction|TryStartMatch))

(event Custom|RefreshAliveCounts
  (Development|PrintString "BR RefreshAlive")
  (bind _asbp_br_game_state (Utilities|Casting|CastToBP_BR_GameState (Game|GetGameState)))
  (Variables|/Game/FPS_Controller/Blueprints/Game/BattleRoyale/BP_BR_GameState.BP_BR_GameState_C|SetAlivePlayerCount _asbp_br_game_state (stale _returnvalue)))

(event Custom|SpawnLootAndZone
  (Development|PrintString "BR SpawnLootAndZone (level actors handle loot/zone)"))

(event Custom|TryStartMatch
  (Development|PrintString "BR TryStartMatch")
  (if (Networking|IsServer)
    (if (>= (stale _returnvalue) (Variables|BattleRoyale|GetMinPlayersToStart))
      (CallFunction|StartCountdown))))

(event Custom|StartCountdown
  (Development|PrintString "BR Countdown")
  (bind _asbp_br_game_state (Utilities|Casting|CastToBP_BR_GameState (Game|GetGameState)))
  (Variables|/Game/FPS_Controller/Blueprints/Game/BattleRoyale/BP_BR_GameState.BP_BR_GameState_C|SetMatchPhase _asbp_br_game_state 1)
  (Utilities|FlowControl|Delay (Variables|BattleRoyale|GetCountdownSeconds))
  (CallFunction|BegininMatch))

(event Custom|BeginInMatch
  (Development|PrintString "BR MATCH STARTED")
  (bind _asbp_br_game_state (Utilities|Casting|CastToBP_BR_GameState (Game|GetGameState)))
  (Variables|/Game/FPS_Controller/Blueprints/Game/BattleRoyale/BP_BR_GameState.BP_BR_GameState_C|SetMatchPhase _asbp_br_game_state 2)
  (CallFunction|SpawnLootandZone)
  (CallFunction|RefreshAliveCounts))

(event Custom|OnPlayerEliminated
  (params (VictimController :type Player%20Controller%20Object%20Reference) (KillerController :type Controller%20Object%20Reference))
  (Development|PrintString "BR Player Eliminated")
  (bind _asbp_br_player_state (Utilities|Casting|CastToBP_BR_PlayerState (Variables|/Script/Engine.Controller|GetPlayerState VictimController)))
  (Variables|/Game/FPS_Controller/Blueprints/Game/BattleRoyale/BP_BR_PlayerState.BP_BR_PlayerState_C|SetbEliminated _asbp_br_player_state true)
  (CallFunction|SpectateTeammate VictimController)
  (CallFunction|RefreshAliveCounts))

(event Custom|SpectateTeammate
  (params (DeadController :type Player%20Controller%20Object%20Reference))
  (Development|PrintString "BR Spectating teammate"))

(event Custom|EndMatchWithWinner
  (params (WinningSquadId :type Integer))
  (Development|PrintString "BR MATCH END")
  (bind _asbp_br_game_state (Utilities|Casting|CastToBP_BR_GameState (Game|GetGameState)))
  (Variables|/Game/FPS_Controller/Blueprints/Game/BattleRoyale/BP_BR_GameState.BP_BR_GameState_C|SetMatchPhase _asbp_br_game_state 3)
  (Variables|/Game/FPS_Controller/Blueprints/Game/BattleRoyale/BP_BR_GameState.BP_BR_GameState_C|SetWinnerSquadId _asbp_br_game_state WinningSquadId)
  (Utilities|FlowControl|Delay (Variables|BattleRoyale|GetEndMatchDelay))
  (Game|OpenLevel(byName) "MainMenu"))

(event Custom|ReturnToMenu
  (Game|OpenLevel(byName) "MainMenu"))

(event Custom|EquipKnifeOnly
  (params (ForController :type Player%20Controller%20Object%20Reference))
  (Development|PrintString "BR EquipKnifeOnly"))

(event EventTick
  (params (DeltaSeconds :type Float%20%28single-precision%29)))

(event EventBeginPlay
  (Development|PrintString "BR GameMode: Waiting for players")
  (bind _returnvalue (UserInterface|CreateWidget "/Game/FPS_Controller/Blueprints/Game/BattleRoyale/UI/WBP_BR_Overlay.WBP_BR_Overlay_C"))
  (UserInterface|Viewport|AddtoViewport _returnvalue 0))

(event EventPostLogin
  (params (NewPlayer :type Player%20Controller%20Object%20Reference))
  (CallFunction|AssignSquadtoController NewPlayer))

(event EventInitializeHUDforPlayer
  (params (NewPlayer :type Player%20Controller%20Object%20Reference))
  (Development|PrintString "BR: skip loadout selection - ground loot only"))

(fn ConstructionScript
  (|CallParentFunction))