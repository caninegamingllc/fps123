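; BP_BR_LootSpawner is a battle royale loot point that randomly spawns a weapon pickup at its own transform.
; SpawnLoot runs on BeginPlay when SpawnOnBeginPlay is set, or when the event is called directly.
; Each attempt prints a debug message, rolls against SpawnChance, and on success spawns BP_PickupWeapon and sets Spawned, which this graph never checks.
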(event Custom|SpawnLoot
  (Development|PrintString "BR Loot Spawn attempt")
  (if (< (Math|Random|RandomFloat) (Variables|Loot|GetSpawnChance))
    (Game|SpawnActorfromClass :Class "/Game/FPS_Controller/Blueprints/WeaponPickup/BP_PickupWeapon.BP_PickupWeapon_C" :SpawnTransform (Transformation|GetActorTransform) :CollisionHandlingOverride "Undefined" :TransformScaleMethod "MultiplyWithRoot" :WeaponMesh 0 :WeaponClass 0 :Magazine 0 :WeaponSkin 0 :ExtraMesh 0 :Instigator 0)
    (Variables|Loot|SetbSpawned true)))

(event EventBeginPlay
  (if (Variables|Loot|GetbSpawnOnBeginPlay)
    (CallFunction|SpawnLoot)))

(event Collision|EventActorBeginOverlap
  (params (OtherActor :type Actor%20Object%20Reference)))

(event EventTick
  (params (DeltaSeconds :type Float%20%28single-precision%29)))

(fn ConstructionScript)