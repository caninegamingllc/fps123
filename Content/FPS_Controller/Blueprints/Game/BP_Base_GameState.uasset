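; BP_Base_GameState is a base game state for the FPS controller that spawns and possesses player pawns.
; SpawnPlayer spawns the game mode's default pawn at the first PlayerStart found, adjusting for collision, then has the given controller possess it.
; Stub functions for game mode widgets, match objectives and a menu check, which returns false, form the rest of the class.
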(event EventSpawnPlayer
  (params (PlayerController :type Player%20Controller%20Object%20Reference))
  ;[0 0 0] Spawn Player
  (bind _outactors (Actor|GetAllActorsOfClass "/Script/Engine.PlayerStart"))
  (bind _returnvalue (Game|SpawnActorfromClass (Variables|/Script/Engine.GameModeBase|GetDefaultPawnClass (Game|GetGameMode)) (Transformation|GetActorTransform (Utilities|Array|Get(acopy) _outactors)) "AdjustIfPossibleButAlwaysSpawn" "SelectDefaultAtRuntime" 0 0))
  (Pawn|Possess PlayerController _returnvalue))

(fn ConstructionScript)

(fn GetGameModeWidgets
  (return 0 0 0))

(fn GetMatchObjectives
  (return 0))

(fn IsMenu
  (return false))