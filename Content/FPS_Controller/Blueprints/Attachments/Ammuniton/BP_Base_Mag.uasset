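; BP_Base_Mag is the base magazine attachment Blueprint in the FPS controller, carrying first-person and third-person meshes.
; On BeginPlay it hides the mag_02 bone on both meshes.
; When the attachment replicates, it sends its AmmoPerMag value to its owner through SetMagAmmoMessage.
; Helper functions return either mesh or destroy the first-person component.
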(event EventBeginPlay
  ;[0 0 0 0.5] Begin Play
  (|CallParentFunction)
  (Components|SkinnedMesh|HideBonebyName (Variables|Default|GetFPP) "mag_02" "PBO_None"))

(event EventOnAttachmentReplicated
  ;[0 0 0] Set Mag Ammo
  (Class|BIWeapon|SetMagAmmo(Message) (Components|GetOwner) (Variables|Default|GetAmmoPerMag)))

(fn ConstructionScript
  (|CallParentFunction))

(fn GetFPPMesh
  (return (Variables|Default|GetFPP)))

(fn GetTPPMesh
  (return (Variables|Default|GetTPP)))

(fn DestroyFPPComponent
  (Components|DestroyComponent (Variables|Default|GetFPP)))